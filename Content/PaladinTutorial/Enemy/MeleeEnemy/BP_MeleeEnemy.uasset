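; Melee enemy Blueprint that patrols at random and chases the Paladin player character on sight.
; While the player is unseen, Tick drives a delayed AI move to random reachable nearby points.
; Pawn sensing raises walk speed, moves to the player, then calls MeleeAttack after a random delay.
; A retriggerable delay clears visibility and restores patrol speed shortly after sightings stop.
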(event OnSeePawn(PawnSensingSeePlayer)
  (params (Pawn :type Pawn%20Object%20Reference))
  ;[0 0 0 0.5] Move to player upon seeing
  (bind _aspaladin_character (Utilities|Casting|CastToPaladinCharacter Pawn))
  (Utilities|FlowControl|Sequence
    (:then_0
      (Variables|Default|SetIsPlayerVisible true)
      (Variables|/Script/Engine.CharacterMovementComponent|SetMaxWalkSpeed (Variables|Character|GetCharacterMovement) 6e+02)
      (AI|AIMoveTo self "0, 0, 0" _aspaladin_character 5.0 false
        (:OnSuccess
          (Utilities|FlowControl|Delay (Math|Random|RandomFloatinRange 0.5 1.5))
          (Class|MeleeEnemy|MeleeAttack))))
    (:then_1
      (Utilities|FlowControl|RetriggerableDelay 0.5)
      (Variables|Default|SetIsPlayerVisible false)
      (Variables|/Script/Engine.CharacterMovementComponent|SetMaxWalkSpeed (Variables|Character|GetCharacterMovement) 2e+02))))

(event Custom|PatrolAround
  ;[0 0 0 0.5] Patrolling BP function
  (if (not (Variables|Default|GetIsPlayerVisible))
    (Utilities|FlowControl|Delay (Math|Random|RandomFloatinRange 1.0 3.0))
    (AI|AIMoveTo self (.RandomLocation (AI|Navigation|GetRandomReachablePointinRadius (Transformation|GetActorLocation) 2.5e+03 0 0)) 0 5.0 false
      (:OnSuccess
        (CallFunction|PatrolAround)))))

(event EventBeginPlay)

(event Collision|EventActorBeginOverlap
  (params (OtherActor :type Actor%20Object%20Reference)))

(event EventTick
  (params (DeltaSeconds :type Float%20%28single-precision%29))
  (CallFunction|PatrolAround))

(fn ConstructionScript)